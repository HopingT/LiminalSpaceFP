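; A simple interactive door Blueprint that swings open and closed on Interact and shows a widget while the player is nearby.
; A box overlap toggles the widget for the cached first-person character.
; Interact alternates through a FlipFlop between playing and reversing a Timeline, which lerps the door's relative yaw.
; A boolean guard limits the horror stinger, played at world origin, to the first Timeline update.
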(event `self.ReceiveBeginPlay`
  (bind _asbp_first_person_character (cast `/Game/FirstPerson/Blueprints/BP_FirstPersonCharacter` (`GameplayStatics.GetPlayerCharacter` 0)))
  (set `self.As BP First Person Character` _asbp_first_person_character))

(event `self.Box.OnComponentBeginOverlap`
  (params (OverlappedComponent :type "PrimitiveComponent Object Reference") (OtherActor :type "Actor Object Reference") (OtherComp :type "PrimitiveComponent Object Reference") (OtherBodyIndex :type Integer) (bFromSweep :type Boolean) (SweepResult :type "HitResult Structure (by ref)"))
  (if (== OtherActor (`self.As BP First Person Character`))
    (`SceneComponent.SetVisibility` (`self.Widget`) true false)))

(event `self.Box.OnComponentEndOverlap`
  (params (OverlappedComponent :type "PrimitiveComponent Object Reference") (OtherActor :type "Actor Object Reference") (OtherComp :type "PrimitiveComponent Object Reference") (OtherBodyIndex :type Integer))
  (if (== OtherActor (`self.As BP First Person Character`))
    (`SceneComponent.SetVisibility` (`self.Widget`) false false)))

(event `/Game/Blueprints/bp_InteractiveDoor.Interact`
  (`/Engine/EditorBlueprintResources/StandardMacros.FlipFlop`
    (:`A`
      (bind (_direction _doorrotation) (`Timeline|Timeline` :!label _label)
        (:`Update`
          (`SceneComponent.K2_SetRelativeRotation` (`self.Door`) (`KismetMathLibrary.MakeRotator` 0.0 0.0 (`KismetMathLibrary.Lerp` 0.0 -100.0 _doorrotation)) false false)
          (if (not (`self.b_Sound`))
            (`GameplayStatics.PlaySoundAtLocation` "/Game/LevelPrototyping/Sounds/11L-cinematic_horror_stinger-68792223.11L-cinematic_horror_stinger-68792223" (0.0 0.0 0.0) (struct) 1.0 1.0 0.0 null null null null)
            (set `self.b_Sound` true)))))
    (:`B`
      (goto _label :!via `Reverse`))))

(fn `UserConstructionScript`)